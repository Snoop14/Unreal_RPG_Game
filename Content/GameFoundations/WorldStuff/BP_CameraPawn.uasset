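; BP_CameraPawn is a camera pawn with a spring arm that supports zooming and orbiting and hides actors blocking the view.
; Enhanced Input drives clamped arm length for zoom and feeds shared yaw and clamped-pitch rotation.
; Tick, throttled by a Delay, unhides everything in HiddenActors, then traces from camera to root on the Camera channel.
; A non-Character hit is hidden outright and added to the never-cleared array.
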(event Input|EnhancedActionEvents|EnhancedInputActionIA_CameraZoom
  (params (ActionValue :type Float%20%28double-precision%29) (ElapsedSeconds :type Float%20%28double-precision%29) (TriggeredSeconds :type Float%20%28double-precision%29) (InputAction :type Input%20Action%20Object%20Reference :default "/Game/GameFoundations/Input/Actions/IA_CameraZoom.IA_CameraZoom"))
  (bind _springarm (Variables|Default|GetSpringArm))
  ;[1 1 1] Set Camera Zoom via Mouse Wheel
  (Variables|/Script/Engine.SpringArmComponent|SetTargetArmLength _springarm (Math|Float|Clamp(Float) (+ (* ActionValue -5e+01) (Variables|/Script/Engine.SpringArmComponent|GetTargetArmLength _springarm)) 5e+02 2.5e+03)))

(event Input|EnhancedActionEvents|EnhancedInputActionIA_CameraRotateVertical
  (params (ActionValue :type Float%20%28double-precision%29) (ElapsedSeconds :type Float%20%28double-precision%29) (TriggeredSeconds :type Float%20%28double-precision%29) (InputAction :type Input%20Action%20Object%20Reference :default "/Game/GameFoundations/Input/Actions/IA_CameraRotateVertical.IA_CameraRotateVertical"))
  (bind _springarm (Variables|Default|GetSpringArm))
  (bind _returnvalue (Class|SpringArmComponent|GetTargetRotation _springarm))
  (bind (_roll _pitch _yaw) (Math|Rotator|BreakRotator _returnvalue))
  ;[1 1 1] Adjust Camera's Vertical and Horizontal Rotation
  (:Triggered
    (Variables|Default|SetCamera%20Vertical%20Value ActionValue)
    (Transformation|SetWorldRotation _springarm (Math|Rotator|MakeRotator 0.0 (Math|Float|Clamp(Float) (+ _pitch (Variables|Default|GetCamera%20Vertical%20Value)) -89.0 -1e+01) (+ _yaw (Variables|Default|GetCamera%20Horizontal%20Value))) false false))
  (:Completed
    (Variables|Default|SetCamera%20Vertical%20Value 0.0)))

(event Input|EnhancedActionEvents|EnhancedInputActionIA_CameraRotateHorizontal
  (params (ActionValue :type Float%20%28double-precision%29) (ElapsedSeconds :type Float%20%28double-precision%29) (TriggeredSeconds :type Float%20%28double-precision%29) (InputAction :type Input%20Action%20Object%20Reference :default "/Game/GameFoundations/Input/Actions/IA_CameraRotateHorizontal.IA_CameraRotateHorizontal"))
  (bind _springarm (Variables|Default|GetSpringArm))
  (bind _returnvalue (Class|SpringArmComponent|GetTargetRotation _springarm))
  (bind (_roll _pitch _yaw) (Math|Rotator|BreakRotator _returnvalue))
  ;[1 1 1] Adjust Camera's Vertical and Horizontal Rotation
  (:Triggered
    (Variables|Default|SetCamera%20Horizontal%20Value ActionValue)
    (Transformation|SetWorldRotation _springarm (Math|Rotator|MakeRotator 0.0 (Math|Float|Clamp(Float) (+ _pitch (Variables|Default|GetCamera%20Vertical%20Value)) -89.0 -1e+01) (+ _yaw (Variables|Default|GetCamera%20Horizontal%20Value))) false false))
  (:Completed
    (Variables|Default|SetCamera%20Horizontal%20Value 0.0)))

(event EventBeginPlay)

(event Collision|EventActorBeginOverlap
  (params (OtherActor :type Actor%20Object%20Reference)))

(event EventTick
  (params (DeltaSeconds :type Float%20%28single-precision%29))
  (bind _hidden_actors (Variables|Default|GetHidden%20Actors))
  ;[1 0.2461 0.2567] Hide and Display Objects between the Camera and end point. To be modified, rather than hiding the object completely, want to make the section transparent
  (Utilities|FlowControl|Delay 0.2)
  (for _array_element _hidden_actors
    (Rendering|SetActorHiddenInGame _array_element false))
  (bind _outhit (Collision|LineTraceByChannel (Transformation|GetWorldLocation (Variables|Default|GetMain%20Camera)) (Transformation|GetWorldLocation (Variables|Default|GetDefaultSceneRoot)) "TraceTypeQuery2" false 0 "ForDuration"))
  (if (Utilities|IsValid (.HitActor (Collision|BreakHitResult _outhit)))
    (Utilities|Casting|CastToCharacter (.HitActor (Collision|BreakHitResult _outhit))
      (:CastFailed
        (Rendering|SetActorHiddenInGame (.HitActor (Collision|BreakHitResult _outhit)) true)
        (Utilities|Array|Add _hidden_actors (.HitActor (Collision|BreakHitResult _outhit)))))))

(fn ConstructionScript)