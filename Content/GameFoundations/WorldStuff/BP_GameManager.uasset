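; BP_GameManager coordinates map travel and switching between exploration and combat.
; OpenNewMap stores a spawn transform and loads the level; PrepareNewMap finds the map's BP_GridManager, binds cell clicks and spawns the party on cells it returns.
; A game state routes clicks and stride requests to the grid manager, handled only during Exploration.
; Starting combat or exploration sets that state and notifies the Combat or Exploration manager, and ending combat resumes exploration.
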(event Custom|Open%20New%20Map
  (params (Level :type World%20Soft%20Object%20Reference) (Spawn%20Location :type Vector) (Spawn%20Rotation :type Rotator))
  (Variables|SpawnDetails|SetSpawn%20Location Spawn%20Location)
  (Variables|SpawnDetails|SetSpawn%20Rotation Spawn%20Rotation)
  (Game|OpenLevel(byObjectReference) Level))

(event Custom|Request%20Stride
  (params (Creature :type BP%20Base%20Creature%20Object%20Reference))
  (switch Utilities|FlowControl|Switch|SwitchonEGameState (Variables|Default|GetCurrent%20Game%20State)
    (:NewEnumerator0
      (Default|DetermineGridPath (Variables|Managers|GetGrid%20Manager) (Variables|/Game/GameFoundations/Characters/BP_BaseCreature.BP_BaseCreature_C|GetCurrent%20Grid%20Cell Creature)))))

(event Custom|Start%20Combat
  (Variables|Default|SetCurrent%20Game%20State "NewEnumerator1")
  (Default|EnterCombatMode (Variables|Managers|GetCombat%20Manager)))

(event Custom|Handle%20Cell%20Clicked
  (switch Utilities|FlowControl|Switch|SwitchonEGameState (Variables|Default|GetCurrent%20Game%20State)
    (:NewEnumerator0
      (Development|PrintString "Game Manager is Handling Cell Click")
      (Default|ExplorationBasicEvent (Variables|Managers|GetGrid%20Manager) (Variables|/Game/GameFoundations/Characters/BP_BaseCreature.BP_BaseCreature_C|GetCurrent%20Grid%20Cell (Variables|/Game/GameFoundations/WorldStuff/BP_PartyManager.BP_PartyManager_C|GetMain%20Character (Variables|Managers|GetParty%20Manager)))))))

(event Custom|Start%20Exploration
  (Variables|Default|SetCurrent%20Game%20State "NewEnumerator0")
  (Default|EnterExplorationMode (Variables|Managers|GetExploration%20Manager)))

(event Custom|End%20Combat
  (CallFunction|StartExploration))

(event Custom|Prepare%20New%20Map
  (params (Player%20Camera :type Pawn%20Object%20Reference))
  (bind _party_manager (Variables|Managers|GetParty%20Manager))
  ;[1 1 1] Get the Grid Manager in the map
  (bind _outactors (Actor|GetAllActorsOfClass "/Game/GameFoundations/GridStuff/BP_GridManager.BP_GridManager_C"))
  (bind _output_get (Variables|Managers|SetGrid%20Manager (Utilities|Array|Get(acopy) _outactors)))
  (Development|PrintString (Utilities|GetObjectName (Utilities|Array|Get(acopy) _outactors)))
  (EventDispatchers|BindEventtoCellClicktoGameManager _output_get (delegate Custom|Handle%20Cell%20Clicked))
  ;[1 1 1] This function currently does not do anything.
  (bind _player_locations (Default|GetPlayerLocations _party_manager))
  (bind _actual_locations (Default|GettheGridCellsforSpawn (Variables|Managers|GetGrid%20Manager) (Variables|SpawnDetails|GetSpawn%20Location) _player_locations))
  (Default|SpawnPlayerCharacters _party_manager _actual_locations Player%20Camera))

(event EventBeginPlay)

(event Collision|EventActorBeginOverlap
  (params (OtherActor :type Actor%20Object%20Reference)))

(event EventTick
  (params (DeltaSeconds :type Float%20%28single-precision%29)))

(fn ConstructionScript)