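; BP_PartyManager spawns the player's party character into the world, currently just the main character.
; SpawnPlayerCharacters creates a BP_PlayerCharacter slightly above the first spawn location and applies MainCharacterData from BP_GameInstance.
; It stores the passed-in camera and attaches it to follow that character, snapping location while keeping relative rotation.
; GetPlayerLocations is an empty stub, and the event graph holds no logic.
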(event Custom|CustomEvent)

(event EventBeginPlay)

(event Collision|EventActorBeginOverlap
  (params (OtherActor :type Actor%20Object%20Reference)))

(event EventTick
  (params (DeltaSeconds :type Float%20%28single-precision%29)))

(fn ConstructionScript)

(fn SpawnPlayerCharacters
  (params (Spawn%20Locations :type Array%20of%20BP%20Grid%20Cell%20Object%20References) (Player%20Cam :type Pawn%20Object%20Reference))
  (Variables|Default|SetPlayer%20Camera Player%20Cam)
  ;[1 1 1 1 22] Spawn a Player Character at the first Grid Cell and set the Character's data to the Main Character. Then Attach the Camera to that character.
  (bind _returnvalue (Game|SpawnActorfromClass "/Game/GameFoundations/Characters/PlayerCharacters/BP_PlayerCharacter.BP_PlayerCharacter_C" (Math|Transform|MakeTransform (+ (Transformation|GetActorLocation (Utilities|Array|Get(acopy) Spawn%20Locations)) "0.000000,0.000000,90.000000")) "AlwaysSpawn" "MultiplyWithRoot" 0 0))
  (bind _asbp_game_instance (Utilities|Casting|CastToBP_GameInstance (Game|GetGameInstance)))
  (Default|SetCharacterData _returnvalue (Variables|/Game/GameFoundations/Characters/PlayerCharacters/BP_GameInstance.BP_GameInstance_C|GetMain%20Character%20Data _asbp_game_instance))
  (Transformation|AttachActorToActor (Variables|Default|GetPlayer%20Camera) 0 "None" "SnapToTarget" "KeepRelative" "KeepRelative" true))

(fn GetPlayerLocations
  (return 0))