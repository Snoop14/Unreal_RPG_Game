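; Base item actor that can register itself with the grid cell at its location in the world.
; On BeginPlay it creates and stores a dynamic outline material instance for highlighting, though this graph does not apply it.
; IteminWorldEvent runs a short vertical object trace through the root and, if it hits a BP_GridCell, passes the item to that cell's AddToCell.
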(event Custom|Item%20in%20World%20Event
  (bind _defaultsceneroot (Variables|Default|GetDefaultSceneRoot))
  (bind _returnvalue (Transformation|GetWorldLocation _defaultsceneroot))
  (bind _outhit (Collision|LineTraceForObjects (+ _returnvalue "0.000000,0.000000,5.000000") (- _returnvalue "0.000000,0.000000,5.000000") (Utilities|Array|MakeArray "ObjectTypeQuery7") false 0 "None"))
  (bind _asbp_grid_cell (Utilities|Casting|CastToBP_GridCell (.HitActor (Collision|BreakHitResult _outhit))))
  (Default|AddtoCell _asbp_grid_cell self))

(event EventBeginPlay
  (bind _returnvalue (Rendering|Material|CreateDynamicMaterialInstance "/Game/Materials/Outline_Mat.Outline_Mat" "None" "None" :!class /Script/Engine.KismetMaterialLibrary))
  (Variables|Default|SetDynamic%20Highlight%20Mat _returnvalue))

(event Collision|EventActorBeginOverlap
  (params (OtherActor :type Actor%20Object%20Reference)))

(event EventTick
  (params (DeltaSeconds :type Float%20%28single-precision%29)))

(fn ConstructionScript)