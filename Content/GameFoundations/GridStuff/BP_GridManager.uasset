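; Grid manager actor that spawns BP_GridCells on static surfaces, relays their clicks and looks up character spawn cells.
; GenerateGrid line-traces a 3D lattice, tilts cells to surface normals and fills two-way position/cell maps.
; DetermineGridPath runs A* over those maps with an octile-style heuristic, allowing diagonals and one-level height steps, rejecting trace-blocked moves.
; CalculateMoveCost separately prices movement with alternating diagonal costs; editor test events colour paths.
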(event Custom|Stride%20Path%20Event
  (params (Start%20Cell :type BP%20Grid%20Cell%20Object%20Reference) (Target%20Cell :type BP%20Grid%20Cell%20Object%20Reference) (Available%20Movement :type Integer) (Next%20Diagonal :type Boolean))
  (Movement|DetermineGridPath Start%20Cell Target%20Cell))

(event Custom|HandleCellClicked
  (params (Grid%20Cell :type BP%20Grid%20Cell%20Object%20Reference))
  (Development|PrintString "Handling cell Clicked")
  (Default|CallCellClicktoWorld))

(event Custom|Editor%20Test%20One%20Cell
  (bind _test_cellpath_array (Variables|Default|GetTest%20CellPath%20Array))
  ;[1 0.78 0] Code to check if one cell exists. To Be Deleted
  (Utilities|Array|Clear _test_cellpath_array)
  (Utilities|Array|Add _test_cellpath_array (.Value (Utilities|Map|Find (Variables|Default|GetPositionsToCells) "2.000000,0.000000,0.000000")))
  (Movement|ColourGridPath _test_cellpath_array))

(event Custom|Editor%20Test%20Path
  (bind _positionstocells (Variables|Default|GetPositionsToCells))
  ;[1 0.7221 0] Handle creating a path from one cell to another. To be used elsewhere and then deleted
  (bind _cells_path (Movement|DetermineGridPath (.Value (Utilities|Map|Find :TargetMap _positionstocells)) (.Value (Utilities|Map|Find _positionstocells "9.000000,5.000000,2.000000"))))
  (Movement|ColourGridPath _cells_path))

(event EventBeginPlay
  (InitiateGrid|GenerateGrid))

(event Collision|EventActorBeginOverlap
  (params (OtherActor :type Actor%20Object%20Reference)))

(event EventTick
  (params (DeltaSeconds :type Float%20%28single-precision%29)))

(fn ConstructionScript)

(fn GenerateGrid
  (bind _returnvalue (Class|KismetMathLibrary|VectorForward))
  (bind _cellsize (Variables|Default|GetCellSize))
  ;[1 1 1] Start with clearing the two maps of Cells and Positions
  (Utilities|Map|Clear (Variables|Default|GetCellsToPositions))
  (Utilities|Map|Clear (Variables|Default|GetPositionsToCells))
  ;[1 1 1] Loop through the X, Y, and Z values to get the positions.
  (for _index (range 0 (Variables|Default|GetSizeX))
    (for _index_2 (range 0 (Variables|Default|GetSizeY))
      (for _index_3 (range 0 (Variables|Default|GetSizeZ))
        ;[0.924 0 0 1 24] Checks if there is an object where the grid cell is located.
        ; THIS NEEDS TO BE CHANGED:
        ; May want to spawn in all grid cells even sky, water, and underground cells, but without the cell visualiser?
        ; - Too many objects will be spawned however. Attempt with only floor spawns first!
        ; Cells may need to check for walls nearby and allow for climbing?
        ; - Difficult to check for, maybe have walls that affect nearest cells?
        (bind (_outhit _returnvalue_2) (Collision|LineTraceForObjects (+ (+ (Math|Vector|MakeVector (* _cellsize _index) (* _cellsize _index_2) (* _cellsize _index_3)) (Transformation|GetActorLocation)) "0.000000,0.000000,60.000000") (- (+ (Math|Vector|MakeVector (* _cellsize _index) (* _cellsize _index_2) (* _cellsize _index_3)) (Transformation|GetActorLocation)) "0.000000,0.000000,40.000000") (Utilities|Array|MakeArray "ObjectTypeQuery1") false 0 "None"))
        ;;[1 1 1] Hit something. And didn't start in the floor
        (if _returnvalue_2
          (if (not (.bInitialOverlap (Collision|BreakHitResult _outhit)))
            ;[1 1 1] Spawns the actual Grid Cells and adds them to the two maps for the cells and position
            (bind _returnvalue_3 (Game|SpawnActorfromClass "/Game/GameFoundations/GridStuff/BP_GridCell.BP_GridCell_C" (Math|Transform|MakeTransform (+ (.ImpactPoint (Collision|BreakHitResult _outhit)) "0.000000,0.000000,0.100000") (Math|Rotator|MakeRotator (.Roll (Math|Rotator|BreakRotator (Math|Rotator|MakeRotationfromAxes (Math|Vector|Normalize (- _returnvalue (* (.Normal (Collision|BreakHitResult _outhit)) (Math|Vector|DotProduct _returnvalue (.Normal (Collision|BreakHitResult _outhit)))))) (Math|Vector|Normalize (Math|Vector|CrossProduct (.Normal (Collision|BreakHitResult _outhit)) (Math|Vector|Normalize (- _returnvalue (* (.Normal (Collision|BreakHitResult _outhit)) (Math|Vector|DotProduct _returnvalue (.Normal (Collision|BreakHitResult _outhit)))))))) (.Normal (Collision|BreakHitResult _outhit))))) (.Pitch (Math|Rotator|BreakRotator (Math|Rotator|MakeRotationfromAxes (Math|Vector|Normalize (- _returnvalue (* (.Normal (Collision|BreakHitResult _outhit)) (Math|Vector|DotProduct _returnvalue (.Normal (Collision|BreakHitResult _outhit)))))) (Math|Vector|Normalize (Math|Vector|CrossProduct (.Normal (Collision|BreakHitResult _outhit)) (Math|Vector|Normalize (- _returnvalue (* (.Normal (Collision|BreakHitResult _outhit)) (Math|Vector|DotProduct _returnvalue (.Normal (Collision|BreakHitResult _outhit)))))))) (.Normal (Collision|BreakHitResult _outhit))))) 0.0)) "AlwaysSpawn" "MultiplyWithRoot" 0 0))
            (EventDispatchers|BindEventtoCellClickedtoManager _returnvalue_3 (EventDispatchers|CreateEvent :!event Custom|HandleCellClicked))
            (Utilities|Map|Add (Variables|Default|GetPositionsToCells) (Math|Vector|MakeVector (Math|Conversions|ToFloat(Integer) _index) (Math|Conversions|ToFloat(Integer) _index_2) (Math|Conversions|ToFloat(Integer) _index_3)) _returnvalue_3)
            (Utilities|Map|Add (Variables|Default|GetCellsToPositions) _returnvalue_3 (Math|Vector|MakeVector (Math|Conversions|ToFloat(Integer) _index) (Math|Conversions|ToFloat(Integer) _index_2) (Math|Conversions|ToFloat(Integer) _index_3))))))))
  (return))

(fn CalculateMoveCost
  (params (Start%20Cell :type BP%20Grid%20Cell%20Object%20Reference) (Target%20Cell :type BP%20Grid%20Cell%20Object%20Reference) (Diagonal%20Next :type Boolean))
  (bind _returnvalue (Transformation|GetActorLocation Start%20Cell))
  (bind _returnvalue_2 (Transformation|GetActorLocation Target%20Cell))
  (bind (_x _y) (Math|Vector|BreakVector _returnvalue))
  (bind (_x_2 _y_2) (Math|Vector|BreakVector _returnvalue_2))
  (bind _returnvalue_3 (- _x _x_2))
  (bind _returnvalue_4 (- _y _y_2))
  (bind _returnvalue_5 (Math|Float|Absolute(Float) _returnvalue_3))
  (bind _returnvalue_6 (Math|Float|Absolute(Float) _returnvalue_4))
  (bind _returnvalue_7 (Math|Float|Min(Float) _returnvalue_5 _returnvalue_6))
  (bind _output_get (LocalVariables|SetDiagonal%20Next%20var Diagonal%20Next))
  (LocalVariables|SetCell%20Moves (- (Math|Float|Max(Float) _returnvalue_5 _returnvalue_6) _returnvalue_7))
  (for _index (range 0 (Math|Float|Truncate _returnvalue_7))
    (if _output_get
      (LocalVariables|SetDiagonal%20Next%20var false)
      (LocalVariables|SetCell%20Moves (+ (LocalVariables|GetCell%20Moves) 2.0))
      (else
        (LocalVariables|SetDiagonal%20Next%20var true)
        (LocalVariables|SetCell%20Moves (+ (LocalVariables|GetCell%20Moves) 1.0)))))
  (return (* (Math|Float|Truncate (LocalVariables|GetCell%20Moves)) 5) (LocalVariables|GetDiagonal%20Next%20var)))

(fn DetermineGridPath
  (params (Start%20Cell :type BP%20Grid%20Cell%20Object%20Reference) (Target%20Cell :type BP%20Grid%20Cell%20Object%20Reference))
  (bind _celltocost (Utilities|Struct|MakeCellToCost Start%20Cell "0.000000,0.000000,0.000000"))
  (bind _found_path (LocalVariables|GetFound%20Path))
  (bind _open_cells (LocalVariables|GetOpen%20Cells))
  (bind _open_cells_2 (LocalVariables|GetOpen%20Cells))
  (bind _newcellpositions (LocalVariables|GetNewCellPositions))
  (bind _newcellpositionstriple (LocalVariables|GetNewCellPositionsTriple))
  (Utilities|Set|Clear (LocalVariables|GetChecked%20Cells))
  (Utilities|Array|Clear (LocalVariables|GetFound%20Path))
  (Utilities|Map|Clear (LocalVariables|GetClosed%20Cells))
  (Utilities|Map|Clear _open_cells)
  (Utilities|Map|Add _open_cells _celltocost _celltocost)
  (while (> (Utilities|Map|Length _open_cells) 0)
    (LocalVariables|SetLowest%20Cost%20Cell (Utilities|Struct|MakeCellToCost 0 "99999999.000000,0.000000,0.000000"))
    (bind _keys (Utilities|Map|Keys _open_cells))
    ;[1 1 1] Find the Cell with the lowest f cost
    (bind _array_element (Utilities|Array|ForEachLoopwithBreak _keys)
      (:LoopBody
        (if (< (.X (Math|Vector|BreakVector (.FGHCost (Utilities|Struct|BreakCellToCost _array_element)))) (.X (Math|Vector|BreakVector (.FGHCost (Utilities|Struct|BreakCellToCost (LocalVariables|GetLowest%20Cost%20Cell))))))
          (LocalVariables|SetLowest%20Cost%20Cell _array_element)))
      (:Completed
        ;[1 1 1] Add cell to Closed Cells and remove from Open Cells
        (Utilities|Map|Add (LocalVariables|GetClosed%20Cells) (LocalVariables|GetLowest%20Cost%20Cell) (.Value (Utilities|Map|Find _open_cells_2 (LocalVariables|GetLowest%20Cost%20Cell))))
        (Utilities|Map|Remove _open_cells_2 (LocalVariables|GetLowest%20Cost%20Cell))
        (if (== Target%20Cell (.Cell (Utilities|Struct|BreakCellToCost (LocalVariables|GetLowest%20Cost%20Cell))))
          ;[1 1 1] True means we got to the cell, time to backtrack. Backtrack via using the value of the closed map to find the parent cell.
          (Utilities|Array|Clear _found_path)
          (Utilities|Array|Add _found_path (.Cell (Utilities|Struct|BreakCellToCost (LocalVariables|GetLowest%20Cost%20Cell))))
          (while (!= (.Cell (Utilities|Struct|BreakCellToCost (LocalVariables|GetLowest%20Cost%20Cell))) Start%20Cell)
            (Utilities|Array|Add _found_path (.Cell (Utilities|Struct|BreakCellToCost (.Value (Utilities|Map|Find (LocalVariables|GetClosed%20Cells) (LocalVariables|GetLowest%20Cost%20Cell))))))
            (LocalVariables|SetLowest%20Cost%20Cell (.Value (Utilities|Map|Find (LocalVariables|GetClosed%20Cells) (LocalVariables|GetLowest%20Cost%20Cell)))))
          (return _found_path)
          (else
            ;[1 1 1] Add the surrounding positions to an array to check them for cells
            (Utilities|Array|Clear _newcellpositions)
            (Utilities|Array|Add _newcellpositions (+ (.Value (Utilities|Map|Find (Variables|Default|GetCellsToPositions) (.Cell (Utilities|Struct|BreakCellToCost (LocalVariables|GetLowest%20Cost%20Cell))))) "1.000000,0.000000,0.000000"))
            (Utilities|Array|Add _newcellpositions (+ (.Value (Utilities|Map|Find (Variables|Default|GetCellsToPositions) (.Cell (Utilities|Struct|BreakCellToCost (LocalVariables|GetLowest%20Cost%20Cell))))) "1.000000,1.000000,0.000000"))
            (Utilities|Array|Add _newcellpositions (+ (.Value (Utilities|Map|Find (Variables|Default|GetCellsToPositions) (.Cell (Utilities|Struct|BreakCellToCost (LocalVariables|GetLowest%20Cost%20Cell))))) "0.000000,1.000000,0.000000"))
            (Utilities|Array|Add _newcellpositions (+ (.Value (Utilities|Map|Find (Variables|Default|GetCellsToPositions) (.Cell (Utilities|Struct|BreakCellToCost (LocalVariables|GetLowest%20Cost%20Cell))))) "-1.000000,1.000000,0.000000"))
            (Utilities|Array|Add _newcellpositions (+ (.Value (Utilities|Map|Find (Variables|Default|GetCellsToPositions) (.Cell (Utilities|Struct|BreakCellToCost (LocalVariables|GetLowest%20Cost%20Cell))))) "-1.000000,0.000000,0.000000"))
            (Utilities|Array|Add _newcellpositions (+ (.Value (Utilities|Map|Find (Variables|Default|GetCellsToPositions) (.Cell (Utilities|Struct|BreakCellToCost (LocalVariables|GetLowest%20Cost%20Cell))))) "-1.000000,-1.000000,0.000000"))
            (Utilities|Array|Add _newcellpositions (+ (.Value (Utilities|Map|Find (Variables|Default|GetCellsToPositions) (.Cell (Utilities|Struct|BreakCellToCost (LocalVariables|GetLowest%20Cost%20Cell))))) "0.000000,-1.000000,0.000000"))
            (Utilities|Array|Add _newcellpositions (+ (.Value (Utilities|Map|Find (Variables|Default|GetCellsToPositions) (.Cell (Utilities|Struct|BreakCellToCost (LocalVariables|GetLowest%20Cost%20Cell))))) "1.000000,-1.000000,0.000000"))
            ;[1 1 1] Add the three potential positions of a nearby cell to an array to check (parallel, above, below)
            (for _array_element_2 (LocalVariables|GetNewCellPositions)
              (Utilities|Array|Clear _newcellpositionstriple)
              (Utilities|Array|Add _newcellpositionstriple _array_element_2)
              (Utilities|Array|Add _newcellpositionstriple (+ _array_element_2 "0.000000,0.000000,1.000000"))
              (Utilities|Array|Add _newcellpositionstriple (- _array_element_2 "0.000000,0.000000,1.000000"))
              ;[1 1 1] Check the cells in the array and ensure it isn't in checked Cells. Then check if cell should be added to algorithm and calculate fgh costs. Add the cell to the Checked Cells set and the Open Cells map
              (bind _array_element_3 (Utilities|Array|ForEachLoopwithBreak (LocalVariables|GetNewCellPositionsTriple) :!label _label)
                (:LoopBody
                  (if (.ReturnValue (Utilities|Map|Find (Variables|Default|GetPositionsToCells) _array_element_3))
                    (if (Utilities|Set|Contains (LocalVariables|GetChecked%20Cells) (.Value (Utilities|Map|Find (Variables|Default|GetPositionsToCells) _array_element_3)))
                      (goto _label Break)
                      (else
                        (bind (_add_cell _fgh_cost) (Movement|CalculateFCost (.Value (Utilities|Map|Find (Variables|Default|GetPositionsToCells) _array_element_3)) (LocalVariables|GetLowest%20Cost%20Cell) Target%20Cell))
                        (if _add_cell
                          (Utilities|Set|Add (LocalVariables|GetChecked%20Cells) (.Value (Utilities|Map|Find (Variables|Default|GetPositionsToCells) _array_element_3)))
                          (Utilities|Map|Add (LocalVariables|GetOpen%20Cells) (Utilities|Struct|MakeCellToCost (.Value (Utilities|Map|Find (Variables|Default|GetPositionsToCells) _array_element_3)) _fgh_cost) (LocalVariables|GetLowest%20Cost%20Cell))
                          (goto _label Break)
                          (else
                            (goto _label Break)))))))))))))))

(fn CalculateFCost
  (params (Current%20Cell :type BP%20Grid%20Cell%20Object%20Reference) (Parent%20Cell :type Cell%20to%20Cost%20Structure) (Target%20Cell :type BP%20Grid%20Cell%20Object%20Reference))
  (bind (_cell _fghcost) (Utilities|Struct|BreakCellToCost Parent%20Cell))
  (bind _cellstopositions (Variables|Default|GetCellsToPositions))
  (bind _value (Utilities|Map|Find _cellstopositions Current%20Cell))
  (bind _value_2 (Utilities|Map|Find _cellstopositions Target%20Cell))
  (bind (_x _y _z) (Math|Vector|BreakVector _value_2))
  (bind (_x_2 _y_2 _z_2) (Math|Vector|BreakVector _value))
  (bind _returnvalue (- _x_2 _x))
  (bind _returnvalue_2 (- _y_2 _y))
  (bind _returnvalue_3 (Math|Float|Absolute(Float) _returnvalue))
  (bind _returnvalue_4 (Math|Float|Absolute(Float) _returnvalue_2))
  (bind _returnvalue_5 (Collision|LineTraceByChannel (+ (Transformation|GetWorldLocation (Variables|/Script/Engine.Actor|GetRootComponent _cell)) "0.000000,0.000000,40.000000") (+ (Transformation|GetWorldLocation (Variables|/Script/Engine.Actor|GetRootComponent Current%20Cell)) "0.000000,0.000000,40.000000") "TraceTypeQuery1" false 0 "None"))
  (if _returnvalue_5
    (return false "0, 0, 0")
    (else
      ;[1 1 1] G value = parent cell + 1
      (bind _output_get (LocalVariables|Setg%20value (+ (.Y (Math|Vector|BreakVector _fghcost)) 1.0)))
      ;[1 1 1] H Value = D * (dx + dy) + (D2 - 2 * D) * min(dx, dy)     D = 1, dx = abs(cell.x - target.x), dy = abs(cell.y - target.y), D2 = sqrt(2)
      ; Modified = (dx + dy + dz) + (D2 - 2) * min(dx, dy)   dz = abs(cell.z - target.z)
      (bind _output_get_2 (LocalVariables|Seth%20value (+ (+ _returnvalue_3 _returnvalue_4 (Math|Float|Absolute(Float) (- _z_2 _z))) (* (Math|Float|Min(Float) _returnvalue_3 _returnvalue_4) (- (Math|Float|Sqrt 2.0) 2.0)))))
      ;[1 1 1] f value = g + h
      (bind _output_get_3 (LocalVariables|Setf%20value (+ _output_get _output_get_2)))
      (return true (Math|Vector|MakeVector _output_get_3 _output_get _output_get_2)))))

(fn ColourGridPath
  (params (Cell%20Path :type Array%20of%20BP%20Grid%20Cell%20Object%20References))
  (for _array_element Cell%20Path
    (Default|UpdateGridMaterial _array_element (Math|Color|MakeColor 0 255 0 100))))

(fn GettheGridCellsforSpawn
  (params (Base%20Location :type Vector) (Relative%20Locations :type Array%20of%20Vectors))
  (bind _positionstocells (Variables|Default|GetPositionsToCells))
  (bind _grid_locations (LocalVariables|GetGrid%20Locations))
  ;[1 1 1] Gets the base location and other spawn locations to get all Grid Cells to spawn characters at.
  (Utilities|Array|Clear _grid_locations)
  (Utilities|Array|Add _grid_locations (.Value (Utilities|Map|Find _positionstocells Base%20Location)))
  (for _array_element Relative%20Locations
    (Utilities|Array|Add _grid_locations (.Value (Utilities|Map|Find _positionstocells (+ Base%20Location _array_element)))))
  (return _grid_locations))