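; BP_GridCell is a clickable grid cell actor that highlights under the cursor and tracks the items it contains.
; At BeginPlay it creates one dynamic material instance shared by its four edge meshes.
; CellCollision cursor events tint that material cyan on hover and white on exit, and clicks pass the cell to a manager.
; Helper functions add items to ContainedItems without duplicates and remove them.
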(event OnBeginCursorOver(CellCollision)
  (params (TouchedComponent :type Primitive%20Component%20Object%20Reference))
  (CallFunction|UpdateGridMaterial (Math|Color|MakeColor 255 255 0 100)))

(event OnEndCursorOver(CellCollision)
  (params (TouchedComponent :type Primitive%20Component%20Object%20Reference))
  (CallFunction|UpdateGridMaterial (Math|Color|MakeColor 255 255 255 100)))

(event OnClicked(CellCollision)
  (params (TouchedComponent :type Primitive%20Component%20Object%20Reference) (ButtonPressed :type Key%20Structure :default "None"))
  (Default|CallCellClickedtoManager self))

(event EventBeginPlay
  (bind _returnvalue (Rendering|Material|CreateDynamicMaterialInstance "/Game/Materials/GridCell_Mat.GridCell_Mat" "None" "None" :!class /Script/Engine.KismetMaterialLibrary))
  (bind _output_get (Variables|Default|SetDynamicMaterial _returnvalue))
  (Rendering|Material|SetMaterial (Variables|Default|GetEdge_Back) 0 _output_get)
  (Rendering|Material|SetMaterial (Variables|Default|GetEdge_Front) 0 _output_get)
  (Rendering|Material|SetMaterial (Variables|Default|GetEdge_Left) 0 _output_get)
  (Rendering|Material|SetMaterial (Variables|Default|GetEdge_Right) 0 _output_get))

(event Collision|EventActorBeginOverlap
  (params (OtherActor :type Actor%20Object%20Reference)))

(event EventTick
  (params (DeltaSeconds :type Float%20%28single-precision%29)))

(fn ConstructionScript)

(fn UpdateGridMaterial
  (params (NewParam :type Color%20Structure))
  (Rendering|Material|SetVectorParameterValue (Variables|Default|GetDynamicMaterial) "Main Color" (Math|Conversions|ToLinearColor(Color) NewParam) :!class /Script/Engine.MaterialInstanceDynamic))

(fn AddtoCell
  (params (New%20Object :type BP%20Base%20Item%20Object%20Reference))
  (bind _contained_items (Variables|Default|GetContained%20Items))
  (if (Utilities|Set|Contains _contained_items New%20Object)
    (return)
    (else
      (Utilities|Set|Add _contained_items New%20Object))))

(fn RemovefromCell
  (params (Remove%20Object :type BP%20Base%20Item%20Object%20Reference))
  (Utilities|Set|Remove (Variables|Default|GetContained%20Items) Remove%20Object))