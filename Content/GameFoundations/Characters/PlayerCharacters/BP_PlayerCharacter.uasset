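; BP_PlayerCharacter is a player character Blueprint that holds a character's identity and its place on a grid.
; Its SetCharacterData event takes character data and a grid cell, storing the cell as the current one and copying the character name and max HP into variables.
; The default BeginPlay, overlap and Tick events are disabled, and the construction script only calls its parent.
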(event Custom|Set%20Character%20Data
  (params (Character%20Data :type Character%20Data%20Structure) (Grid%20Cell :type BP%20Grid%20Cell%20Object%20Reference))
  (bind (_charactername _level _exp _keyattribute _classproficiency _classdc _ancestry _heritage _size _background _class _attributes _maxhp) (Utilities|Struct|BreakCharacterData Character%20Data))
  (Variables|Default|SetCurrent%20Grid%20Cell Grid%20Cell)
  (Variables|Default|SetName _charactername)
  (Variables|Default|SetMax%20HP _maxhp))

(event EventBeginPlay
  (|CallParentFunction) ; This node is disabled and will not be called.\nDrag off pins to build functionality.
)

(event Collision|EventActorBeginOverlap
  (params (OtherActor :type Actor%20Object%20Reference))
  (|CallParentFunction OtherActor) ; This node is disabled and will not be called.\nDrag off pins to build functionality.
)

(event EventTick
  (params (DeltaSeconds :type Float%20%28single-precision%29))
  (|CallParentFunction DeltaSeconds) ; This node is disabled and will not be called.\nDrag off pins to build functionality.
)

(fn ConstructionScript
  (|CallParentFunction))